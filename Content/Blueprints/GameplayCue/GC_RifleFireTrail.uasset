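; GC_RifleFireTrail is a burst gameplay cue that aims the rifle fire trail effect from a BP_ZZCharacter.
; On burst, it projects a distant point along player 0's view direction, without tracing for hits.
; It converts that point into the character's Muzzle local space and sets it as the BeamEnd vector parameter on the spawned FX.
; The loop returns after the first FX component.
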(fn `OnBurst`
  (params (Target :type "Actor Object Reference") (Parameters :type "GameplayCueParameters Structure (by ref)") (SpawnResults :type "GameplayCueNotify_SpawnResult Structure (by ref)"))
  (bind _asbp_zzcharacter (cast `/Game/Characters/ZZCharacter/BP_ZZCharacter` Target))
  (for _array_element (`.FxSystemComponents` (break `GameplayCueNotify_SpawnResult` SpawnResults))
    (bind (_location _rotation) (`Controller.GetPlayerViewPoint` (`GameplayStatics.GetPlayerController` _asbp_zzcharacter)))
    (`FXSystemComponent.SetVectorParameter` _array_element "BeamEnd" (`KismetMathLibrary.InverseTransformLocation` (`SceneComponent.K2_GetComponentToWorld` (`/Game/Characters/ZZCharacter/BP_ZZCharacter.Muzzle` _asbp_zzcharacter)) (+ _location (* (`KismetMathLibrary.GetForwardVector` _rotation) 20000.0))))
    (return)))