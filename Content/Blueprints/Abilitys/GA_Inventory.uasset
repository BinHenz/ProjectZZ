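; Gameplay Ability that toggles the player's inventory display on and off.
; On activation it commits, casts the avatar to BP_ZZCharacter, and shows or hides the inventory through its ACZZInventoryComponent based on the component's Showing flag.
; It then ends immediately, using EndAbility on the server and EndAbilityLocally otherwise.
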(event `self.K2_ActivateAbility`
  (`self.K2_CommitAbility`)
  (bind _asbp_zzcharacter (cast `/Game/Characters/ZZCharacter/BP_ZZCharacter` (`self.GetAvatarActorFromActorInfo`)))
  (bind _ac_zzinventorycomponent (`/Game/Characters/ZZCharacter/BP_ZZCharacter.AC_ZZInventoryComponent` _asbp_zzcharacter))
  (if (`/Game/Blueprints/Component/AC_ZZInventoryComponent.Showing` _ac_zzinventorycomponent)
    (`/Game/Blueprints/Component/AC_ZZInventoryComponent.F_HideInventory` _ac_zzinventorycomponent)
    (else
      (`/Game/Blueprints/Component/AC_ZZInventoryComponent.F_ShowInventory` _ac_zzinventorycomponent)))
  (if (`KismetSystemLibrary.IsServer`)
    (`self.K2_EndAbility`)
    (else
      (`self.K2_EndAbilityLocally`))))