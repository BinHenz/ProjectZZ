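; Behavior tree task that picks a random patrol destination for a BP_ZZZombie.
; It sets the zombie to patrol walk speed, then queries navigation for a random reachable point within the patrol radius around the pawn.
; The point is written to the PatrolLoaction blackboard key, falling back to the pawn's current location if none is found.
; The task succeeds either way and fails only when the pawn is not a BP_ZZZombie.
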(event `self.ReceiveExecuteAI`
  (params (OwnerController :type "AIController Object Reference") (ControlledPawn :type "Pawn Object Reference"))
  (bind _returnvalue (`Actor.K2_GetActorLocation` ControlledPawn))
  (bind (_randomlocation _returnvalue_2) (`NavigationSystemV1.K2_GetRandomReachablePointInRadius` _returnvalue (`self.PatrolRadius`) null null))
  (bind _asbp_zzzombie (cast `/Game/Characters/ZZZombie/BP_ZZZombie` ControlledPawn)
    (:`then`
      (`/Game/Characters/ZZZombie/BP_ZZZombie.UpdateWalkSpeed` _asbp_zzzombie (`self.Normal Walk Speed (Patrol)`))
      (if _returnvalue_2
        (`BTFunctionLibrary.SetBlackboardValueAsVector` (`self.PatrolLoaction`) _randomlocation)
        (else
          (`BTFunctionLibrary.SetBlackboardValueAsVector` (`self.PatrolLoaction`) _returnvalue)))
      (`self.FinishExecute` true))
    (:`CastFailed`
      (`self.FinishExecute` false))))