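; BP_MasterItem is a world item that can be picked up through an overlapping actor's AC_ZZInventoryComponent.
; On overlap with InteractCollision, it either adds itself to the inventory and destroys itself when AutoPickUp is set, or registers as the pickup target and shows the interaction prompt.
; End overlap unregisters it, hiding the prompt when no items remain.
; The construction script optionally enables mesh physics and removes RotatingMovement when unused.
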(event `self.InteractCollision.OnComponentBeginOverlap`
  (params (OverlappedComponent :type "PrimitiveComponent Object Reference") (OtherActor :type "Actor Object Reference") (OtherComp :type "PrimitiveComponent Object Reference") (OtherBodyIndex :type Integer) (bFromSweep :type Boolean) (SweepResult :type "HitResult Structure (by ref)"))
  (bind _returnvalue (`self.GetComponentByClass` OtherActor "/Game/Blueprints/Component/AC_ZZInventoryComponent.AC_ZZInventoryComponent_C"))
  (if (`KismetSystemLibrary.DoesImplementInterface` _returnvalue "/Game/Blueprints/Component/BPI_InventoryInterface.BPI_InventoryInterface_C")
    (if (`/Game/Blueprints/Component/AC_ZZInventoryComponent.AutoPickUp` _returnvalue)
      (`/Game/Blueprints/Component/AC_ZZInventoryComponent.F_AddItemToInventory` _returnvalue self)
      (`self.K2_DestroyActor`)
      (else
        (`KismetArrayLibrary.Array_Add` (`/Game/Blueprints/Component/AC_ZZInventoryComponent.OverlappingItem` _returnvalue) self)
        (set `/Game/Blueprints/Component/AC_ZZInventoryComponent.ItemToPickUp` self _returnvalue)
        (`/Game/Blueprints/Component/AC_ZZInventoryComponent.SetInteractionVisibility` _returnvalue true)))))

(event `self.InteractCollision.OnComponentEndOverlap`
  (params (OverlappedComponent :type "PrimitiveComponent Object Reference") (OtherActor :type "Actor Object Reference") (OtherComp :type "PrimitiveComponent Object Reference") (OtherBodyIndex :type Integer))
  (bind _returnvalue (`self.GetComponentByClass` OtherActor "/Game/Blueprints/Component/AC_ZZInventoryComponent.AC_ZZInventoryComponent_C"))
  (bind _overlappingitem (`/Game/Blueprints/Component/AC_ZZInventoryComponent.OverlappingItem` _returnvalue))
  (`/Engine/EditorBlueprintResources/StandardMacros.IsValid` OtherActor
    (:`Is Valid`
      (if (`KismetSystemLibrary.DoesImplementInterface` _returnvalue "/Game/Blueprints/Component/BPI_InventoryInterface.BPI_InventoryInterface_C")
        (`KismetArrayLibrary.Array_RemoveItem` _overlappingitem self)
        (if (not (> (`KismetArrayLibrary.Array_Length` _overlappingitem) 0))
          (`/Game/Blueprints/Component/AC_ZZInventoryComponent.SetInteractionVisibility` _returnvalue false))))))

(fn `UserConstructionScript`
  (bind _itemstaticmesh (`self.ItemStaticMesh`))
  (if (`self.UsePhysics`)
    (`PrimitiveComponent.SetSimulatePhysics` _itemstaticmesh true)
    (`PrimitiveComponent.SetCollisionEnabled` _itemstaticmesh "QueryAndPhysics"))
  (if (not (`self.UseRotatingMovement`))
    (`ActorComponent.K2_DestroyComponent` (`self.RotatingMovement`))))